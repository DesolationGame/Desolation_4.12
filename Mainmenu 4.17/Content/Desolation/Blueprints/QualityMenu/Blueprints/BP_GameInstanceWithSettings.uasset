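; Game instance Blueprint that owns the game's settings system and serves as its settings interface.
; On Init it creates a settings wrapper tied to a save slot, passing itself as the interface, and stores it for retrieval.
; Interface functions execute console commands and apply audio channel volumes, each returning an unused dummy bool.
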(event EventInit
  (bind _game_settings_wrapper (CallFunction|InitGameSettings "GameSettingsSave" 0 self))
  (Variables|Default|SetGame%20Settings%20Wrapper _game_settings_wrapper))

(fn GetSettingsInstance
  (return (Variables|Default|GetGame%20Settings%20Wrapper)))

(fn RunConsoleCommand
  (params (Console%20Command :type String))
  (Development|ExecuteConsoleCommand Console%20Command)
  (return false) ; Ignore output. It is not used.\n\nInterface function includes\na dummy bool output so it\nwill show up in blueprints\nthat implements interface.
)

(fn UpdateAudioChannel
  (params (Audio%20Channel :type EAudioType%20Enum :default "NewEnumerator4") (Volume :type Float%20%28single-precision%29))
  (CallFunction|ApplyAudioChannel Audio%20Channel Volume self)
  (return false) ; Ignore output. It is not used.\n\nInterface function includes\na dummy bool output so it\nwill show up in blueprints\nthat implements interface.
)