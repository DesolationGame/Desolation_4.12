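; Analog axis key input for the keybinding utilities in the quality menu, overriding the parent's current-state query.
; It reads the controller's analog key state and keeps only the positive or negative half, as a positive magnitude.
; That value is returned as the axis value and thresholded into a digital down state.
; Just-pressed and just-released come from comparing it with the stored previous value, which is not updated here.
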(fn KeyInputCurrentState
  (params (Controller :type Player%20Controller%20Object%20Reference))
  (bind _self self)
  (bind _self_2 self)
  (bind _self_3 self)
  (bind _analog_previous_axis_value (Variables|/Game/QualityMenu/Blueprints/Util/Keybinding/BP_KeyInput.BP_KeyInput_C|GetAnalog%20Previous%20Axis%20Value _self_2))
  (bind _analog_use_negative_axis (Variables|/Game/QualityMenu/Blueprints/Util/Keybinding/BP_KeyInput.BP_KeyInput_C|GetAnalog%20Use%20Negative%20Axis _self_3))
  (bind _key_input (Variables|/Game/QualityMenu/Blueprints/Util/Keybinding/BP_KeyInput.BP_KeyInput_C|GetKey%20Input _self))
  (bind _returnvalue (Class|PlayerController|GetInputAnalogKeyState Controller _key_input))
  (bind _returnvalue_2 (Math|Float|Min(Float) _returnvalue 0.0))
  (bind _returnvalue_3 (Math|Float|Max(Float) _returnvalue 0.0))
  (bind _returnvalue_4 (Math|Float|Absolute(Float) _returnvalue_2))
  (bind _returnvalue_5 (Math|Float|SelectFloat _returnvalue_4 _returnvalue_3 _analog_use_negative_axis))
  ;[1 1 1] Analog Axis Input
  (return _returnvalue_5 (>= _returnvalue_5 0.1) (and (>= _returnvalue_5 0.1) (< _analog_previous_axis_value 0.1)) (and (< _returnvalue_5 0.1) (>= _analog_previous_axis_value 0.1))))