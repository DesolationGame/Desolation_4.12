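; BP_KeyMapping is one named, scaled key binding in the keybinding utilities, holding a primary and a secondary BP_KeyCombination.
; Its current state sums both combinations' axis values times Scale and merges their active, pressed and released flags.
; The merge avoids a repeat press or early release when the two combinations overlap.
; Saving, loading and reverting to defaults are delegated to both combinations.
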(fn InitKeyMapping
  (params (Key%20Mapping :type S%20Key%20Mapping%20Structure))
  (bind (_name _scale _cantbenone _primarycombination _secondarycombination) (Utilities|Struct|BreakSKeyMapping Key%20Mapping))
  (bind _self self)
  (bind _self_2 self)
  (Variables|Default|SetName _name)
  (Variables|Default|SetScale _scale)
  (Utilities|FlowControl|Sequence
    (:then_0
      (bind _returnvalue (Game|ConstructObjectfromClass "/Game/QualityMenu/Blueprints/Util/Keybinding/BP_KeyCombination.BP_KeyCombination_C" _self_2 _self_2))
      (bind _combination (Default|InitKeyCombination _returnvalue _name _cantbenone _primarycombination))
      (Variables|Default|SetPrimary%20Combination _combination))
    (:then_1
      (bind _returnvalue_2 (Game|ConstructObjectfromClass "/Game/QualityMenu/Blueprints/Util/Keybinding/BP_KeyCombination.BP_KeyCombination_C" _self _self))
      (bind _combination_2 (Default|InitKeyCombination _returnvalue_2 _name _cantbenone _secondarycombination))
      (Variables|Default|SetSecondary%20Combination _combination_2))
    (:then_2
      (return self))))

(fn KeyMappingCurrentState
  (params (Player%20Controller :type Player%20Controller%20Object%20Reference))
  (Utilities|FlowControl|Sequence
    (:then_0
      (bind (_axis_value _is_active _just_pressed _just_released) (Default|KeyCombinationCurrentState (Variables|Default|GetPrimary%20Combination) Player%20Controller false))
      (LocalVariables|SetMapping%20Axis%20Value (+ _axis_value (LocalVariables|GetMapping%20Axis%20Value))))
    (:then_1
      (bind (_axis_value_2 _is_active_2 _just_pressed_2 _just_released_2) (Default|KeyCombinationCurrentState (Variables|Default|GetSecondary%20Combination) Player%20Controller false))
      (LocalVariables|SetMapping%20Axis%20Value (+ _axis_value_2 (LocalVariables|GetMapping%20Axis%20Value))))
    (:then_2
      (return (* (Variables|Default|GetScale) (LocalVariables|GetMapping%20Axis%20Value)) (.Is_Active (|Mapping_State _is_active _just_pressed _just_released _is_active_2 _just_pressed_2 _just_released_2)) (.Just_Pressed (|Mapping_State _is_active _just_pressed _just_released _is_active_2 _just_pressed_2 _just_released_2)) (.Just_Released (|Mapping_State _is_active _just_pressed _just_released _is_active_2 _just_pressed_2 _just_released_2))) ; Return combination of\nprimary and secondary
    )))

(fn SaveKeyMapping
  (params (Game%20Settings :type BP%20Game%20Settings%20Object%20Reference) (KeySave :type S%20Key%20Action%20Save%20Structure%20%28by%20ref%29))
  (bind _returnvalue (|Copy KeySave))
  (bind _scale (Variables|Default|GetScale))
  (bind _name (Variables|Default|GetName))
  (Utilities|FlowControl|Sequence
    (:then_0
      (bind _structout (Utilities|Struct|SetmembersinSKeyActionSave _returnvalue _name _scale true))
      (Default|SaveKeyCombination (Variables|Default|GetPrimary%20Combination) Game%20Settings _structout))
    (:then_1
      (bind _structout_2 (Utilities|Struct|SetmembersinSKeyActionSave _returnvalue _name _scale false))
      (Default|SaveKeyCombination (Variables|Default|GetSecondary%20Combination) Game%20Settings _structout_2))))

(fn LoadKeyMapping
  (params (Game%20Settings :type BP%20Game%20Settings%20Object%20Reference) (Action%20Name :type String) (Category :type String))
  (bind _name (Variables|Default|GetName))
  (Default|LoadKeyCombination (Variables|Default|GetPrimary%20Combination) Game%20Settings Action%20Name Category _name true)
  (Default|LoadKeyCombination (Variables|Default|GetSecondary%20Combination) Game%20Settings Action%20Name Category _name false))

(fn ReverttoDefaultKeyMapping
  (bind _primary_combination (Variables|Default|GetPrimary%20Combination))
  (bind _secondary_combination (Variables|Default|GetSecondary%20Combination))
  (Default|ReplaceKeyCombination _primary_combination (Variables|/Game/QualityMenu/Blueprints/Util/Keybinding/BP_KeyCombination.BP_KeyCombination_C|GetDefault%20Combination _primary_combination))
  (Default|ReplaceKeyCombination _secondary_combination (Variables|/Game/QualityMenu/Blueprints/Util/Keybinding/BP_KeyCombination.BP_KeyCombination_C|GetDefault%20Combination _secondary_combination)))