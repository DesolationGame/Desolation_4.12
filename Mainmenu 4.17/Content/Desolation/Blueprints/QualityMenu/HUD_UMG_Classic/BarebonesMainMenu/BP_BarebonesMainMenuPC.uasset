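; BP_BarebonesMainMenuPC is the player controller for the barebones main menu.
; On BeginPlay it creates the menu widget, hands it the ActionManager, shows the cursor and switches to UI-only input focused on the widget.
; It forwards every key press to the ActionManager and uses the "Update Keybinding" input axis event to tick it, apparently to support key rebinding.
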(event EventBeginPlay
  (bind _returnvalue (UserInterface|CreateWidget "/Game/QualityMenu/HUD_UMG_Classic/BarebonesMainMenu/WB_BarebonesMainMenu.WB_BarebonesMainMenu_C" self (Variables|Default|GetActionManager)))
  (UserInterface|Viewport|AddtoViewport _returnvalue 0)
  (Input|SetInputModeUIOnly self _returnvalue false)
  (Variables|Default|SetbShowMouseCursor true))

(event Input|AxisEvents|InputAxisUpdateKeybinding
  (params (AxisValue :type Float%20%28single-precision%29))
  (Default|TickActionManager (Variables|Default|GetActionManager)))

(event Input|KeyboardEvents|AnyKey
  (params (Key :type Key%20Structure :default "AnyKey"))
  (:Pressed
    (Default|AnyKeyPress (Variables|Default|GetActionManager) Key)))

(fn ConstructionScript)